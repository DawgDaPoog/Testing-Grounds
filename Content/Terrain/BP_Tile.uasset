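; BP_Tile is a terrain tile for an infinite terrain game that scatters randomized props and gates the player with a barrier.
; On BeginPlay it locks and calls PlaceActors for rocks, artifacts, pillars and other props with count, radius and scale ranges.
; The player overlapping LockingVolume turns the barrier green and passable; leaving turns it red and solid.
; Overlapping OnCollisionDestroy makes InfiniteTerainGameMode spawn another tile, then destroys this one.
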(event OnComponentEndOverlap(LockingVolume)
  (params (OverlappedComponent :type Primitive%20Component%20Object%20Reference) (OtherActor :type Actor%20Object%20Reference) (OtherComp :type Primitive%20Component%20Object%20Reference) (OtherBodyIndex :type Integer))
  (Utilities|IsPlayerActor OtherActor)
  (CallFunction|Lock))

(event OnComponentBeginOverlap(LockingVolume)
  (params (OverlappedComponent :type Primitive%20Component%20Object%20Reference) (OtherActor :type Actor%20Object%20Reference) (OtherComp :type Primitive%20Component%20Object%20Reference) (OtherBodyIndex :type Integer) (bFromSweep :type Boolean) (SweepResult :type Hit%20Result%20Structure%20%28by%20ref%29))
  (Utilities|IsPlayerActor OtherActor)
  (CallFunction|Unlock))

(event OnComponentBeginOverlap(OnCollisionDestroy)
  (params (OverlappedComponent :type Primitive%20Component%20Object%20Reference) (OtherActor :type Actor%20Object%20Reference) (OtherComp :type Primitive%20Component%20Object%20Reference) (OtherBodyIndex :type Integer) (bFromSweep :type Boolean) (SweepResult :type Hit%20Result%20Structure%20%28by%20ref%29))
  (Utilities|IsPlayerActor OtherActor)
  (bind _asinfinite_terain_game_mode (Utilities|Casting|CastToInfiniteTerainGameMode (Game|GetGameMode)))
  (Default|SpawnTile _asinfinite_terain_game_mode)
  (Actor|DestroyActor))

(event EventBeginPlay
  (CallFunction|Lock)
  (Class|Tile|PlaceActors "/Game/MeshesBlueprints/SM_Agelsjon_Rock_Boulder_1_BP.SM_Agelsjon_Rock_Boulder_1_BP_C" 1 4 1e+02 1.5 3.0)
  (Class|Tile|PlaceActors "/Game/MeshesBlueprints/Artifacts_Node7_BP.Artifacts_Node7_BP_C" 2 5 1e+02 0.7 4.0)
  (Class|Tile|PlaceActors "/Game/MeshesBlueprints/PrimeHelixer_BP.PrimeHelixer_BP_C" 1 4 1.2e+03 0.2 0.4)
  (Class|Tile|PlaceActors "/Game/MeshesBlueprints/SM_Angelsjon_Cylinder_BP.SM_Angelsjon_Cylinder_BP_C" 2 4 2e+02 1.0 2.0)
  (Class|Tile|PlaceActors "/Game/MeshesBlueprints/Static_Pillar_Trim_C_BP.Static_Pillar_Trim_C_BP_C" 1 3 4e+02 0.7 1.3))

(event Collision|EventActorBeginOverlap
  (params (OtherActor :type Actor%20Object%20Reference)))

(event EventTick
  (params (DeltaSeconds :type Float%20%28single-precision%29)))

(fn ConstructionScript)

(fn GetAttachLocation
  (return (Transformation|GetWorldTransform (Variables|Default|GetSpawnPoint))))

(fn Unlock
  (bind _barrier (Variables|Default|GetBarrier))
  (Collision|SetCollisionEnabled _barrier "NoCollision")
  (Rendering|Material|SetMaterial _barrier 0 "/Game/Terrain/MI_Barrier_Green.MI_Barrier_Green"))

(fn Lock
  (bind _barrier (Variables|Default|GetBarrier))
  (Collision|SetCollisionEnabled _barrier "QueryAndPhysics")
  (Rendering|Material|SetMaterial _barrier 0 "/Game/Terrain/MI_Barrier_Red.MI_Barrier_Red"))